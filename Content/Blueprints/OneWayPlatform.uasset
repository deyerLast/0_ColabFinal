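; One-way platform for a Paper2D level that ColabGameCharacter can land on from above and drop through by crouching.
; Sprite collision starts disabled and turns on when the character begins overlapping the actor while moving downward and not crouching.
; It turns off again when the character leaves CollisionComponent, or on any Tick where player 0 is crouching.
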(event `self.ReceiveBeginPlay`
  (`PrimitiveComponent.SetCollisionEnabled` (`PaperSpriteActor.RenderComponent` (`self.PaperSprite`)) "NoCollision" :!label _label))

(event `self.ReceiveTick`
  (params (DeltaSeconds :type "Float (single-precision)"))
  (bind _ascolab_game_character (cast `ColabGameCharacter` (`GameplayStatics.GetPlayerCharacter` 0)))
  (if (`ColabGameCharacter.crouching` _ascolab_game_character)
    (goto _label)))

(event `self.ReceiveActorBeginOverlap`
  (params (OtherActor :type "Actor Object Reference"))
  ;[1 1 1] Overlap Begin
  (bind _ascolab_game_character (cast `ColabGameCharacter` OtherActor))
  (if (> 0.0 (.z (`self.GetVelocity` OtherActor)))
    (if (not (`ColabGameCharacter.crouching` _ascolab_game_character))
      (`PrimitiveComponent.SetCollisionEnabled` (`PaperSpriteActor.RenderComponent` (`self.PaperSprite`)) "QueryAndPhysics"))))

(event `self.CollisionComponent.OnComponentEndOverlap`
  (params (OverlappedComponent :type "PrimitiveComponent Object Reference") (OtherActor :type "Actor Object Reference") (OtherComp :type "PrimitiveComponent Object Reference") (OtherBodyIndex :type Integer))
  ;[1 1 1] Overlap End
  (cast `ColabGameCharacter` OtherActor)
  (goto _label))

(fn `UserConstructionScript`)