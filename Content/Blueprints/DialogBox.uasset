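; DialogBox is a Paper2D sprite actor that shows a dialog box image for a limited time.
; BeginPlay assigns the configured Sprite to its PaperSprite component.
; PopUp resets the elapsed timer and stores the requested show duration.
; Tick accumulates time, keeping the sprite visible and IsVisible true only until that duration elapses.
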(event `self.ReceiveBeginPlay`
  (`PaperSpriteComponent.SetSprite` (`self.PaperSprite`) (`self.Sprite`)))

(event `self.ReceiveTick`
  (params (DeltaSeconds :type "Float (single-precision)"))
  (bind _output_get (set `self.Time` (+ DeltaSeconds (`self.Time`))))
  (bind _returnvalue (> (`self.VisibleTime`) _output_get))
  (`SceneComponent.SetVisibility` (`self.PaperSprite`) _returnvalue false)
  (set `self.IsVisible` _returnvalue))

(fn `PopUp`
  (params (ShowTime :type "Float (double-precision)"))
  (set `self.Time` 0.0)
  (set `self.VisibleTime` ShowTime))

(fn `UserConstructionScript`)