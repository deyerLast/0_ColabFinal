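; Ferryman NPC that ends the game in a win when the player brings at least 50 coins.
; Box overlap toggles input, so Interact plays a sound, checks the player's inventory and toggles either the win dialog or the default dialog.
; Tick bobs the box with a sine offset and, once won with the win dialog hidden, calls DisplayWinScreen every frame, creating the menu, showing the cursor and disabling player input.
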(event `self.ReceiveActorBeginOverlap`
  (params (OtherActor :type "Actor Object Reference")))

(event `self.ReceiveTick`
  (params (DeltaSeconds :type "Float (single-precision)"))
  (bind _box (`self.Box`))
  ;[1 1 1] Hover Code - Alex
  (bind _output_get (set `self.HoverTime` (+ (* DeltaSeconds (`self.HoverSpeed`)) (`self.HoverTime`))))
  (`SceneComponent.K2_SetWorldLocation` _box (`KismetMathLibrary.MakeVector` (.x (`SceneComponent.K2_GetComponentLocation` _box)) (.y (`SceneComponent.K2_GetComponentLocation` _box)) (+ (.z (`SceneComponent.K2_GetComponentLocation` _box)) (* (`KismetMathLibrary.Sin` _output_get) (`self.HoverHeight`)))) false false)
  ;[1 1 1] If the game is won. Check if the dialog disapeared and activate the win screen! - Alex
  (if (and (not (`/Game/Blueprints/DialogBox.IsVisible` (`self.WinDialog`))) (`self.WonTheGame`))
    (`self.DisplayWinScreen`) ; -JD
  ))

(event `self.Box.OnComponentBeginOverlap`
  (params (OverlappedComponent :type "PrimitiveComponent Object Reference") (OtherActor :type "Actor Object Reference") (OtherComp :type "PrimitiveComponent Object Reference") (OtherBodyIndex :type Integer) (bFromSweep :type Boolean) (SweepResult :type "HitResult Structure (by ref)"))
  ;[1 1 1] Enable input when player overlaps our collision - Alex
  (cast `ColabGameCharacter` OtherActor)
  (`self.EnableInput` (`GameplayStatics.GetPlayerController` 0)))

(event `InputAction|Interact`
  (params (Key :type "Key Structure"))
  (bind _windialog (`self.WinDialog`))
  (bind _dialog (`self.Dialog`))
  ;[1 1 1] Input Logic. Checks if player has 50 coins.- Alex
  (:`Pressed`
    (bind _ascolab_char_bp (cast `/Game/2DSideScrollerCPP/Blueprints/ColabCharBP` (`GameplayStatics.GetPlayerCharacter` 0)))
    (bind _inventoryref (`/Game/2DSideScrollerCPP/Blueprints/ColabCharBP.InventoryRef` _ascolab_char_bp))
    (bind (_success_ _index) (`/Game/InventorySystem/BluePrints/BP_Inventory.HasItem?` _inventoryref "/Game/InventorySystem/BluePrints/ItemClasses/CoinItem.CoinItem_C"))
    (if _success_
      (if (>= (`/Game/InventorySystem/BluePrints/BP_Inventory.GetAmountAtIndex` _inventoryref _index) 50)
        ;[1 1 1] True: Enable/Disable Alternate Dialog! - Alex
        (set `self.WonTheGame` true)
        (if (`/Game/Blueprints/DialogBox.IsVisible` _windialog)
          (`/Game/Blueprints/DialogBox.PopUp` _windialog 0.0)
          (else
            (`/Game/Blueprints/DialogBox.PopUp` _windialog 6.0)))
        (else
          ;[1 1 1] False: Enable/Disable Dialog Popup - Alex
          (if (`/Game/Blueprints/DialogBox.IsVisible` _dialog) :!label _label
            (`/Game/Blueprints/DialogBox.PopUp` _dialog 0.0)
            (else
              (`/Game/Blueprints/DialogBox.PopUp` _dialog 6.0)))))
      (else
        (goto _label)))
    ;[1 1 1] Gave him a noise:)-JD
    (`GameplayStatics.PlaySoundAtLocation` "/Game/Sounds/Ferryman.Ferryman" (`SceneComponent.K2_GetComponentLocation` (`self.PaperFlipbook`)))))

(event `self.Box.OnComponentEndOverlap`
  (params (OverlappedComponent :type "PrimitiveComponent Object Reference") (OtherActor :type "Actor Object Reference") (OtherComp :type "PrimitiveComponent Object Reference") (OtherBodyIndex :type Integer))
  ;[1 1 1] Disable input when player exits our collision - Alex
  (cast `ColabGameCharacter` OtherActor)
  (`self.DisableInput` (`GameplayStatics.GetPlayerController` 0)))

(fn `DisplayWinScreen`
  (bind _returnvalue (`GameplayStatics.GetPlayerController` 0))
  (bind _returnvalue_2 (`|CreateWidget` "/Game/Menus/WInMenu.WInMenu_C"))
  (`UserWidget.AddToViewport` _returnvalue_2 0)
  (set `PlayerController.bShowMouseCursor` true _returnvalue)
  (`self.DisableInput` (`GameplayStatics.GetPlayerCharacter` 0) _returnvalue))

(fn `UserConstructionScript`)