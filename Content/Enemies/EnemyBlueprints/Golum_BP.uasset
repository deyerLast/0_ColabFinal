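; Golum enemy Blueprint that animates a Paper2D flipbook, attacks when the player is in range and dies when health runs out.
; A looping timer opens periodic attack windows, which Tick closes after a delay.
; Tick also snaps yaw to 180-degree steps and feeds state to a flipbook selector, though IsHit is never passed in.
; Attacking Sword overlaps call OnHitComp and trigger a damage sound; death plays a sound, then destroys the actor.
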(event `self.ReceiveActorBeginOverlap`
  (params (OtherActor :type "Actor Object Reference"))
  (bind _assword (cast `/Game/2DSideScroller/Sprites/PlayerAssets/Sword` OtherActor))
  (if (`/Game/2DSideScroller/Sprites/PlayerAssets/Sword.Attacking` _assword)
    (`self.OnHitComp`)
    (set `self.IsHit?` true)))

(event `self.ReceiveTick`
  (params (DeltaSeconds :type "Float (single-precision)"))
  (bind _enemybox (`self.EnemyBox`))
  (bind _returnvalue (`SceneComponent.K2_GetComponentLocation` (`self.EnemyBox`)))
  ;[1 1 1] Added code that locks the rotation! :D  - Alex
  (`SceneComponent.K2_SetWorldRotation` _enemybox (`KismetMathLibrary.MakeRotator` (.roll (`SceneComponent.K2_GetComponentRotation` _enemybox)) (.pitch (`SceneComponent.K2_GetComponentRotation` _enemybox)) (* (`KismetMathLibrary.Round` (/ (.yaw (`SceneComponent.K2_GetComponentRotation` _enemybox)) 180.0)) 180.0)) false false)
  (if (<= (`KismetMathLibrary.VSize` (- (`SceneComponent.K2_GetComponentLocation` (`Character.CapsuleComponent` (`GameplayStatics.GetPlayerCharacter` 0))) (`SceneComponent.K2_GetComponentLocation` (`self.EnemyBox`)))) (`self.AttRange`))
    (if (`self.CanBeAttacking`)
      (set `self.IsAttacking?` true)
      (else
        (set `self.IsAttacking?` false))))
  (bind _output_get (set `self.IsDead?` (<= (`self.Health`) 0.0)))
  (bind _output_get_2 (set `self.IsMoving?` (> (`KismetMathLibrary.VSize` (`self.GetVelocity`)) 0.0)))
  (bind _outbook (`self.Anim State Machine ` false _output_get_2 _output_get (`self.IsAttacking?`)))
  (`PaperFlipbookComponent.SetFlipbook` (`self.PaperFlipbook`) _outbook)
  (if (`self.IsDead?`)
    (`/Engine/EditorBlueprintResources/StandardMacros.DoOnce` false
      (:`Completed`
        (`GameplayStatics.PlaySoundAtLocation` "/Game/Sounds/Golum-Die.Golum-Die" _returnvalue)
        (`KismetSystemLibrary.Delay` 0.75)
        (`self.K2_DestroyActor`)))
    (elif (`self.CanBeAttacking`)
      (`KismetSystemLibrary.Delay` 1.0)
      (set `self.CanBeAttacking` false)
      (elif (`self.IsHit?`)
        (`GameplayStatics.PlaySoundAtLocation` "/Game/Sounds/Golum-Damage.Golum-Damage" _returnvalue)
        (set `self.IsHit?` false)))))

(event `self.ReceiveBeginPlay`
  (`KismetSystemLibrary.K2_SetTimer` null "AttackCountdown" 3.0 true))

(fn `Anim State Machine `
  (params (`IsHit?` :type Boolean) (`IsMoving?` :type Boolean) (`IsDead?` :type Boolean) (`IsAttacking?` :type Boolean))
  (returns (OutBook :type "PaperFlipbook Object Reference"))
  (if `IsDead?`
    (set `self.GolumEnum` "NewEnumerator4")
    (elif `IsAttacking?`
      (set `self.GolumEnum` "NewEnumerator2")
      (elif `IsHit?`
        (set `self.GolumEnum` "NewEnumerator3")
        (elif `IsMoving?`
          (set `self.GolumEnum` "NewEnumerator1")
          (else
            (set `self.GolumEnum` "NewEnumerator0"))))))
  (return (select `/Game/Enemies/EnemyBlueprints/Golum_Enumeration` (`self.GolumEnum`) :`NewEnumerator0` (`self.Golum_Idle`) :`NewEnumerator1` (`self.Golum_Amble`) :`NewEnumerator2` (`self.Golum_Attack`) :`NewEnumerator3` (`self.Golum_Damage`) :`NewEnumerator4` (`self.Golum_Death`))))

(fn `AttackCountdown`
  (set `self.CanBeAttacking` true))

(fn `UserConstructionScript`)