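; Paper2D skeleton enemy that animates by state, reacts to attacking Sword overlaps and destroys itself after a death sound and short delay.
; Tick snaps yaw to half-turns, derives dead, moving and attacking flags, then picks a flipbook through a priority-based state function.
; A looping timer opens short attack windows, used when the player is within range.
; Hits call OnHitComp, but their animation state reuses the amble flipbook, not the damage one.
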(event `self.ReceiveActorBeginOverlap`
  (params (OtherActor :type "Actor Object Reference"))
  (bind _assword (cast `/Game/2DSideScroller/Sprites/PlayerAssets/Sword` OtherActor))
  (if (`/Game/2DSideScroller/Sprites/PlayerAssets/Sword.Attacking` _assword)
    (`self.OnHitComp`)
    (set `self.IsHit?` true)))

(event `self.ReceiveTick`
  (params (DeltaSeconds :type "Float (single-precision)"))
  (bind _enemybox (`self.EnemyBox`))
  (bind _returnvalue (`SceneComponent.K2_GetComponentLocation` (`self.EnemyBox`)))
  (`SceneComponent.K2_SetWorldRotation` _enemybox (`KismetMathLibrary.MakeRotator` (.roll (`SceneComponent.K2_GetComponentRotation` _enemybox)) (.pitch (`SceneComponent.K2_GetComponentRotation` _enemybox)) (* (`KismetMathLibrary.Round` (/ (.yaw (`SceneComponent.K2_GetComponentRotation` _enemybox)) 180.0)) 180.0)) false false)
  (if (<= (`KismetMathLibrary.VSize` (- (`SceneComponent.K2_GetComponentLocation` (`Character.CapsuleComponent` (`GameplayStatics.GetPlayerCharacter` 0))) (`SceneComponent.K2_GetComponentLocation` (`self.EnemyBox`)))) (`self.AttRange`))
    (if (`self.CanBeAttacking?`)
      (set `self.IsAttacking?` true)
      (else
        (set `self.IsAttacking?` false))))
  (bind _output_get (set `self.IsDead?` (<= (`self.Health`) 0.0)))
  (bind _output_get_2 (set `self.IsMoving?` (> (`KismetMathLibrary.VSize` (`self.GetVelocity`)) 0.0)))
  (bind _outbook (`self.Anim State Machine` _output_get (`self.IsHit?`) _output_get_2 (`self.IsAttacking?`)))
  (`PaperFlipbookComponent.SetFlipbook` (`self.PaperFlipbook`) _outbook)
  (if (`self.IsDead?`)
    (`/Engine/EditorBlueprintResources/StandardMacros.DoOnce` false
      (:`Completed`
        (`GameplayStatics.PlaySoundAtLocation` "/Game/Sounds/Skeleton-Die.Skeleton-Die" _returnvalue)
        (`KismetSystemLibrary.Delay` 1.0)
        (`self.K2_DestroyActor`)))
    (elif (`self.CanBeAttacking?`)
      (`KismetSystemLibrary.Delay` 1.0)
      (set `self.CanBeAttacking?` false)
      (elif (`self.IsHit?`)
        (`GameplayStatics.PlaySoundAtLocation` "/Game/Sounds/SKeleton-Damage.Skeleton-Damage" _returnvalue)
        (set `self.IsHit?` false)))))

(event `self.ReceiveBeginPlay`
  (`KismetSystemLibrary.K2_SetTimer` null "AttackCooldown" 3.0 true))

(fn `Anim State Machine`
  (params (`IsDead?` :type Boolean) (`IsHit?` :type Boolean) (`IsMoving?` :type Boolean) (`IsAttacking?` :type Boolean))
  (returns (OutBook :type "PaperFlipbook Object Reference"))
  (if `IsDead?`
    (set `self.SkeletonEnum` "NewEnumerator4")
    (elif `IsAttacking?`
      (set `self.SkeletonEnum` "NewEnumerator1")
      (elif `IsHit?`
        (set `self.SkeletonEnum` "NewEnumerator2")
        (elif `IsMoving?`
          (set `self.SkeletonEnum` "NewEnumerator2")
          (else
            (set `self.SkeletonEnum` "NewEnumerator0"))))))
  (return (select `/Game/Enemies/EnemyBlueprints/Skeleton_Enumeration` (`self.SkeletonEnum`) :`NewEnumerator0` (`self.Skeleton-Idle`) :`NewEnumerator1` (`self.Skeleton-Attack`) :`NewEnumerator2` (`self.Skeleton-Amble`) :`NewEnumerator3` (`self.Skeleton-Damage`) :`NewEnumerator4` (`self.Skeleton-Death`))))

(fn `AttackCooldown`
  (set `self.CanBeAttacking?` true))

(fn `UserConstructionScript`)