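; Slime enemy with flipbook animation that reacts to sword hits and dies when its health runs out.
; Overlap with an attacking Sword calls OnHitComp and flags a hit, which Tick clears after playing the damage sound.
; Tick also snaps yaw to 180-degree steps and picks idle, amble, damage or death flipbooks through a priority-based state function.
; Death plays a sound once, then destroys the actor after a short delay.
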(event `self.ReceiveActorBeginOverlap`
  (params (OtherActor :type "Actor Object Reference"))
  (bind _assword (cast `/Game/2DSideScroller/Sprites/PlayerAssets/Sword` OtherActor))
  (if (`/Game/2DSideScroller/Sprites/PlayerAssets/Sword.Attacking` _assword)
    (`self.OnHitComp`)
    (set `self.IsHit?` true)))

(event `self.ReceiveTick`
  (params (DeltaSeconds :type "Float (single-precision)"))
  (bind _enemybox (`self.EnemyBox`))
  (bind _returnvalue (`SceneComponent.K2_GetComponentLocation` (`self.EnemyBox`)))
  (`SceneComponent.K2_SetWorldRotation` _enemybox (`KismetMathLibrary.MakeRotator` (.roll (`SceneComponent.K2_GetComponentRotation` _enemybox)) (.pitch (`SceneComponent.K2_GetComponentRotation` _enemybox)) (* (`KismetMathLibrary.Round` (/ (.yaw (`SceneComponent.K2_GetComponentRotation` _enemybox)) 180.0)) 180.0)) false false)
  (bind _output_get (set `self.IsDead?` (<= (`self.Health`) 0.0)))
  (bind _output_get_2 (set `self.IsMoving?` (> (`KismetMathLibrary.VSize` (`self.GetVelocity`)) 0.0)))
  (bind _outputflipbook (`self.Anim State Machine ` _output_get_2 (`self.IsHit?`) _output_get))
  (`PaperFlipbookComponent.SetFlipbook` (`self.PaperFlipbook`) _outputflipbook)
  (if (`self.IsDead?`)
    (`/Engine/EditorBlueprintResources/StandardMacros.DoOnce` false
      (:`Completed`
        (`GameplayStatics.PlaySoundAtLocation` "/Game/Sounds/Slime-Death.Slime-Death" _returnvalue)
        (`KismetSystemLibrary.Delay` 1.0)
        (`self.K2_DestroyActor`)))
    (elif (`self.IsHit?`)
      (`GameplayStatics.PlaySoundAtLocation` "/Game/Sounds/Slime-Damage.Slime-Damage" _returnvalue)
      (set `self.IsHit?` false))))

(fn `Anim State Machine `
  (params (`IsMoving?` :type Boolean) (`IsHit?` :type Boolean) (`IsDead?` :type Boolean))
  (returns (OutputFlipbook :type "PaperFlipbook Object Reference"))
  (if `IsDead?`
    (set `self.AnimationState` "NewEnumerator3")
    (elif `IsHit?`
      (set `self.AnimationState` "NewEnumerator2")
      (elif `IsMoving?`
        (set `self.AnimationState` "NewEnumerator1")
        (else
          (set `self.AnimationState` "NewEnumerator0")))))
  (return (select `byte` (`self.AnimationState`) :`0` (`self.Slime_Idle`) :`1` (`self.Slime_Amble`) :`2` (`self.Slime_Damage`) :`3` (`self.Slime_Death`))))

(fn `UserConstructionScript`)