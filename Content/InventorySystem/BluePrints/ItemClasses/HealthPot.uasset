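; HealthPot is a health potion item in the inventory system that heals the player character when it begins play.
; On BeginPlay it casts player character 0 to ColabCharBP and, if Health is below MaxHealth, adds a fixed amount and caps the result at MaxHealth.
; The construction script only calls its parent, and the graph contains no pickup, input or destroy logic.
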(event `self.ReceiveBeginPlay`
  (bind _ascolab_char_bp (cast `/Game/2DSideScrollerCPP/Blueprints/ColabCharBP` (`GameplayStatics.GetPlayerCharacter` 0)))
  (bind _maxhealth (`/Game/2DSideScrollerCPP/Blueprints/ColabCharBP.MaxHealth` _ascolab_char_bp))
  (if (< (`/Game/2DSideScrollerCPP/Blueprints/ColabCharBP.Health` _ascolab_char_bp) _maxhealth)
    (set `self.CharecterHealth` null)
    (bind _ascolab_char_bp_2 (cast `/Game/2DSideScrollerCPP/Blueprints/ColabCharBP` (`GameplayStatics.GetPlayerCharacter` 0)))
    (bind _health (`/Game/2DSideScrollerCPP/Blueprints/ColabCharBP.Health` _ascolab_char_bp_2))
    (set `/Game/2DSideScrollerCPP/Blueprints/ColabCharBP.Health` (+ _health 50.0) _ascolab_char_bp_2)
    (if (>= _health _maxhealth)
      (set `/Game/2DSideScrollerCPP/Blueprints/ColabCharBP.Health` _maxhealth _ascolab_char_bp_2))))

(fn `UserConstructionScript`
  (`parent.UserConstructionScript`))