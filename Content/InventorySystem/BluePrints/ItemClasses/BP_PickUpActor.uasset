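; BP_PickUpActor is a world pickup that adds a configured item and amount to the inventory of a ColabCharBP character that touches it.
; When its Sphere begins overlapping that character, it calls AddItem on the character's InventoryRef.
; On success it keeps any leftover as its new Amount, destroying itself only when nothing remains.
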(event `self.Sphere.OnComponentBeginOverlap`
  (params (OverlappedComponent :type "PrimitiveComponent Object Reference") (OtherActor :type "Actor Object Reference") (OtherComp :type "PrimitiveComponent Object Reference") (OtherBodyIndex :type Integer) (bFromSweep :type Boolean) (SweepResult :type "HitResult Structure (by ref)"))
  (bind _ascolab_char_bp (cast `/Game/2DSideScrollerCPP/Blueprints/ColabCharBP` OtherActor))
  (bind _inventoryref (`/Game/2DSideScrollerCPP/Blueprints/ColabCharBP.InventoryRef` _ascolab_char_bp))
  (`/Engine/EditorBlueprintResources/StandardMacros.IsValid` _inventoryref
    (:`Is Valid`
      (bind (_succes_ _rest) (`/Game/InventorySystem/BluePrints/BP_Inventory.AddItem` _inventoryref (`self.ItemToAdd`) (`self.Amount`)))
      (if _succes_
        (if (> _rest 0)
          (set `self.Amount` _rest)
          (else
            (`self.K2_DestroyActor`)))))))

(fn `UserConstructionScript`)